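; BP_PadBlue is a pad that opens its linked blue door while a blue color cube rests on it.
; Capsule overlap events store the overlapping BP_ColorCube and set a flag, which Tick polls to check the cube's color.
; A blue cube calls BlueOpen every frame, while other colors only print a debug message.
; Any color cube leaving the capsule clears the flag and calls BlueClose.
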(event OnComponentBeginOverlap(Capsule)
  (params (OverlappedComponent :type Primitive%20Component%20Object%20Reference) (OtherActor :type Actor%20Object%20Reference) (OtherComp :type Primitive%20Component%20Object%20Reference) (OtherBodyIndex :type Integer) (bFromSweep :type Boolean) (SweepResult :type Hit%20Result%20Structure%20%28by%20ref%29))
  (bind _asbp_color_cube (Utilities|Casting|CastToBP_ColorCube OtherActor))
  (bind _output_get (Variables|Default|SetIsOverlapped true)))

(event OnComponentEndOverlap(Capsule)
  (params (OverlappedComponent :type Primitive%20Component%20Object%20Reference) (OtherActor :type Actor%20Object%20Reference) (OtherComp :type Primitive%20Component%20Object%20Reference) (OtherBodyIndex :type Integer))
  (Utilities|Casting|CastToBP_ColorCube OtherActor)
  (Variables|Default|SetIsOverlapped false)
  (Default|BlueClose (Variables|Default|GetBlueDoor)))

(event EventTick
  (params (DeltaSeconds :type Float%20%28single-precision%29))
  (if (stale OnComponentBeginOverlap(Capsule) _output_get)
    (if (== (Variables|/Game/Blueprints/BP_ColorCube.BP_ColorCube_C|GetColor (stale OnComponentBeginOverlap(Capsule) _asbp_color_cube)) "Blue")
      (Development|PrintString "Opening Door..." true true "(R=0.000000,G=0.660000,B=1.000000,A=1.000000)" 2.0 "Open")
      (Default|BlueOpen (Variables|Default|GetBlueDoor))
      (else
        (Development|PrintString "Thats not blue." true true "(R=0.000000,G=0.660000,B=1.000000,A=1.000000)" 2.0 "!Blue")))))

(fn ConstructionScript
  (|CallParentFunction))